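; Player pawn for a grid puzzle in which the character melts after a limited number of moves, then the level restarts.
; WASD presses, gated by a cooldown timer, line-trace toward the neighbouring BP_GridPoint and rotate the pawn.
; Non-wall tiles become the target Tick lerps toward; non-final ones count moves and swap in the melted mesh at the limit.
; Physical animation simulates skeletal bodies below ParentBone.
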(event `self.ReceiveTick`
  (params (DeltaSeconds :type "Float (single-precision)"))
  ;[1 1 1] Every frame lerping the position to target position
  (`self.K2_SetActorLocation` (`KismetMathLibrary.VLerp` (`self.K2_GetActorLocation`) (`self.targetPos`) 0.1))
  ;[1 1 1] Restarting level after melting
  (if (`self.melted`)
    (`KismetSystemLibrary.Delay` 1.5)
    (`self.RestartLevel`)))

(event `self.ReceiveBeginPlay`
  (bind _parentbone (`self.parentBone`))
  ;[1 1 1] Setting target position to current position on begin play
  (set `self.targetPos` (`self.K2_GetActorLocation`))
  ;[1 1 1] Physical Animations
  (`PhysicalAnimationComponent.SetSkeletalMeshComponent` (`self.PhysicalAnimation`) (`self.SkeletalMesh`))
  (`PhysicalAnimationComponent.ApplyPhysicalAnimationSettingsBelow` (`self.PhysicalAnimation`) _parentbone (make `PhysicalAnimationData` false 500.0 100.0 1000.0 100.0) false)
  (`SkeletalMeshComponent.SetAllBodiesBelowSimulatePhysics` (`self.SkeletalMesh`) _parentbone true false))

(event `Key|A`
  (params (Key :type "Key Structure"))
  (bind (_returnvalue_x _returnvalue_y _returnvalue_z) (`KismetMathLibrary.BreakVector` (`self.K2_GetActorLocation`)))
  (bind (_returnvalue_x_2 _returnvalue_y_2 _returnvalue_z_2) (`KismetMathLibrary.BreakVector` (`self.K2_GetActorLocation`)))
  ;[1 1 1] A KEY - Move Left
  (:`Pressed`
    (if (`self.canMove`)
      (set `self.canMove` false)
      (`KismetSystemLibrary.K2_SetTimer` null "ResetMove" (`self.moveCooldown`))
      (`self.MovePlayer` (`KismetMathLibrary.MakeVector` _returnvalue_x (+ _returnvalue_y -100.0) _returnvalue_z) (`KismetMathLibrary.MakeVector` _returnvalue_x_2 (+ _returnvalue_y_2 -250.0) _returnvalue_z_2))
      (if (not (`self.melted`))
        (`self.K2_SetActorRotation` (struct :`Yaw` -90.0))))))

(event `Key|W`
  (params (Key :type "Key Structure"))
  (bind (_returnvalue_x _returnvalue_y _returnvalue_z) (`KismetMathLibrary.BreakVector` (`self.K2_GetActorLocation`)))
  (bind (_returnvalue_x_2 _returnvalue_y_2 _returnvalue_z_2) (`KismetMathLibrary.BreakVector` (`self.K2_GetActorLocation`)))
  ;[1 1 1] W KEY - Move Up
  (:`Pressed`
    (if (`self.canMove`)
      (set `self.canMove` false)
      (`KismetSystemLibrary.K2_SetTimer` null "ResetMove" (`self.moveCooldown`))
      (`self.MovePlayer` (`KismetMathLibrary.MakeVector` (+ _returnvalue_x 100.0) _returnvalue_y _returnvalue_z) (`KismetMathLibrary.MakeVector` (+ _returnvalue_x_2 250.0) _returnvalue_y_2 _returnvalue_z_2))
      (if (not (`self.melted`))
        (`self.K2_SetActorRotation` (struct))))))

(event `Key|S`
  (params (Key :type "Key Structure"))
  (bind (_returnvalue_x _returnvalue_y _returnvalue_z) (`KismetMathLibrary.BreakVector` (`self.K2_GetActorLocation`)))
  (bind (_returnvalue_x_2 _returnvalue_y_2 _returnvalue_z_2) (`KismetMathLibrary.BreakVector` (`self.K2_GetActorLocation`)))
  ;[1 1 1] S KEY - Move Down
  (:`Pressed`
    (if (`self.canMove`)
      (set `self.canMove` false)
      (`KismetSystemLibrary.K2_SetTimer` null "ResetMove" (`self.moveCooldown`))
      (`self.MovePlayer` (`KismetMathLibrary.MakeVector` (+ _returnvalue_x -100.0) _returnvalue_y _returnvalue_z) (`KismetMathLibrary.MakeVector` (+ _returnvalue_x_2 -250.0) _returnvalue_y_2 _returnvalue_z_2))
      (if (not (`self.melted`))
        (`self.K2_SetActorRotation` (struct :`Yaw` 180.0))))))

(event `Key|D`
  (params (Key :type "Key Structure"))
  (bind (_returnvalue_x _returnvalue_y _returnvalue_z) (`KismetMathLibrary.BreakVector` (`self.K2_GetActorLocation`)))
  (bind (_returnvalue_x_2 _returnvalue_y_2 _returnvalue_z_2) (`KismetMathLibrary.BreakVector` (`self.K2_GetActorLocation`)))
  ;[1 1 1] D KEY - Move Right
  (:`Pressed`
    (if (`self.canMove`)
      (set `self.canMove` false)
      (`KismetSystemLibrary.K2_SetTimer` null "ResetMove" (`self.moveCooldown`))
      (`self.MovePlayer` (`KismetMathLibrary.MakeVector` _returnvalue_x (+ _returnvalue_y 100.0) _returnvalue_z) (`KismetMathLibrary.MakeVector` _returnvalue_x_2 (+ _returnvalue_y_2 250.0) _returnvalue_z_2))
      (if (not (`self.melted`))
        (`self.K2_SetActorRotation` (struct :`Yaw` 90.0))))))

(fn `MovePlayer`
  (params (Start :type "Vector Structure") (End :type "Vector Structure"))
  ;[1 1 1] Raycast
  (bind _outhit (`KismetSystemLibrary.LineTraceSingle` Start End "TraceTypeQuery3"))
  (if (not (`self.melted`))
    ;[1 1 1] Checking for walls, ice walls, final tile
    (bind _asbp_grid_point (cast `/Game/Blueprints/BP_GridPoint` (`.HitActor` (`GameplayStatics.BreakHitResult` _outhit))))
    (if (`/Game/Blueprints/BP_GridPoint.isWall` _asbp_grid_point)
      (`KismetSystemLibrary.PrintString` "WALL" :!label _label)
      (elif (`/Game/Blueprints/BP_GridPoint.isIceWall` _asbp_grid_point)
        (goto _label)
        (else
          (set `self.targetPos` (`SceneComponent.K2_GetComponentLocation` (`/Game/Blueprints/BP_GridPoint.PlayerLocation` _asbp_grid_point)))
          (if (`/Game/Blueprints/BP_GridPoint.isFinalTile` _asbp_grid_point)
            (`KismetSystemLibrary.PrintString` "YOU WIN")
            (else
              ;[1 1 1] Adding movement and checking for death
              (bind _output_get (set `self.movements` (+ (`self.movements`) 1)))
              (bind _output_get_2 (set `self.melted` (>= _output_get (`self.maxMovements`))))
              (`SceneComponent.SetVisibility` (`self.SkeletalMesh`) (not _output_get_2) false)
              (`SceneComponent.SetVisibility` (`self.MeltedPlayer`) _output_get_2 false))))))))

(fn `ResetMove`
  (locals (time :type "Float (double-precision)"))
  (set `self.canMove` true))

(fn `RestartLevel`
  (bind _returnvalue (`GameplayStatics.GetCurrentLevelName` true))
  (`GameplayStatics.OpenLevel` (`KismetStringLibrary.Conv_StringToName` _returnvalue)))

(fn `UserConstructionScript`)