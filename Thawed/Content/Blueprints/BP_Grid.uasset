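; BP_Grid is a grid actor that builds a square field of BP_GridPoint child actors in its construction script.
; Nested loops over ChunksEachLength add child actor components spaced by ChunkLength, storing each in GridArray and its relative location as a key in GridLocations.
; After clearing and rebuilding, it flags the first point as a wall and calls UpdateType on it.
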(fn `UserConstructionScript`
  (locals (MyGridArray :type "Array of Integer") (GridLocations :type "Map of Vector Structure to Transform Structure") (TempGridLocationKey :type "Vector Structure"))
  (bind _chunklength (`self.ChunkLength`))
  (bind _returnvalue (- (`self.ChunksEachLength`) 1))
  (`KismetArrayLibrary.Array_Clear` (`self.isWall`))
  (`KismetArrayLibrary.Array_Clear` (`self.GridArray`))
  (for _index (range (+ _returnvalue 1))
    (for _index_2 (range (+ _returnvalue 1))
      (bind _returnvalue_2 (* (`KismetMathLibrary.Conv_IntToDouble` _index) _chunklength))
      (bind _returnvalue_3 (* _chunklength (`KismetMathLibrary.Conv_IntToDouble` _index_2)))
      (bind _returnvalue_4 (`AddComponent|NODE_AddChildActorComponent-0` :`RelativeTransform` (`KismetMathLibrary.MakeTransform` (`KismetMathLibrary.MakeVector` _returnvalue_2 _returnvalue_3 1.0))))
      (`KismetArrayLibrary.Array_Add` (`self.GridArray`) _returnvalue_4)
      (bind _output_get (set `local.TempGridLocationKey` (`KismetMathLibrary.MakeVector` _returnvalue_2 _returnvalue_3 1.0)))
      (`BlueprintMapLibrary.Map_Add` (`local.GridLocations`) _output_get)))
  (bind _asbp_grid_point (cast `/Game/Blueprints/BP_GridPoint` (`ChildActorComponent.ChildActor` (`|GetArrayItem` (`self.GridArray`)))))
  (set `/Game/Blueprints/BP_GridPoint.isWall` true _asbp_grid_point)
  (`/Game/Blueprints/BP_GridPoint.UpdateType` _asbp_grid_point))