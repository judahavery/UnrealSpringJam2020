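; Level manager that configures each level at start and handles the transition to the next one.
; On BeginPlay it sets the player pawn's move limit, then either shows the start menu with a cursor on TitleLevel or fades in from a hidden cursor state.
; Tick polls the pawn's LevelComplete flag, then clears it, fades the camera out, waits the transition duration and opens NextLevel by name.
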(event `self.ReceiveBeginPlay`
  ;[1 1 1] Setting Max Movements In Each Level For Player
  (bind _asbp_player_pawn (cast `/Game/Blueprints/BP_PlayerPawn` (`GameplayStatics.GetPlayerPawn` 0)))
  (set `/Game/Blueprints/BP_PlayerPawn.playerMaxMovements` (`self.setPlayerMaxMovements`) _asbp_player_pawn)
  ;[1 1 1] Title Screen UI Setup
  (bind _returnvalue (`GameplayStatics.GetCurrentLevelName` true))
  (bind _output_get (set `self.isTitleScreen` (`KismetStringLibrary.EqualEqual_StrStr` _returnvalue "TitleLevel")))
  (if _output_get
    (bind _returnvalue_2 (`|CreateWidget` "/Game/UserInterface/UI_StartMenu.UI_StartMenu_C"))
    (`UserWidget.AddToViewport` _returnvalue_2 0)
    (set `PlayerController.bShowMouseCursor` true (`GameplayStatics.GetPlayerController` 0))
    (else
      (set `PlayerController.bShowMouseCursor` false (`GameplayStatics.GetPlayerController` 0))
      (`self.FadeInLevel`))))

(event `self.ReceiveTick`
  (params (DeltaSeconds :type "Float (single-precision)"))
  (bind _asbp_player_pawn (cast `/Game/Blueprints/BP_PlayerPawn` (`GameplayStatics.GetPlayerPawn` 0) :!pure true))
  ;[1 1 1] Playing Next Level
  (if (`/Game/Blueprints/BP_PlayerPawn.levelComplete` _asbp_player_pawn)
    (`self.FadeOutLevel`)
    (set `/Game/Blueprints/BP_PlayerPawn.levelComplete` false _asbp_player_pawn)
    (`KismetSystemLibrary.Delay` (`self.LevelTransitionDuration`))
    (`GameplayStatics.OpenLevel` (`self.NextLevel`))))

(fn `FadeInLevel`
  (`PlayerCameraManager.StartCameraFade` :`self` (`GameplayStatics.GetPlayerCameraManager` 0) :`FromAlpha` 1.1 :`ToAlpha` 0.0 :`Duration` (`self.LevelTransitionDuration`) :`bHoldWhenFinished` true))

(fn `FadeOutLevel`
  (`PlayerCameraManager.StartCameraFade` :`self` (`GameplayStatics.GetPlayerCameraManager` 0) :`FromAlpha` 0.0 :`ToAlpha` 1.1 :`Duration` (`self.LevelTransitionDuration`) :`bHoldWhenFinished` true))

(fn `UserConstructionScript`)