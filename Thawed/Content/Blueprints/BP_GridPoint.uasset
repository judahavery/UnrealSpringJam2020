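; Grid tile for a movement puzzle, configured by flags as lock, key, sprout, wall, ice block, finish or final tile.
; Construction script sets component visibility; Tick spins the key and turns the tile into sprout, then wall, as MovementsOnPoint rises.
; Ice blocks scale to MaxMovements, lerp toward targets lowered by ShrinkIceBlock alongside their melt widget, and melt with sound once the player pawn's Movements reach that limit.
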(event `self.ReceiveTick`
  (params (DeltaSeconds :type "Float (single-precision)"))
  (bind _icewall (`self.IceWall`))
  (bind _meltui (`self.MeltUI`))
  ;[1 1 1] TICK
  ;[1 1 1] Rotate Key
  (`self.Rotate` (`self.Key`))
  ;[1 1 1] Checking for changes based on movements per grid point
  (if (== (`self.movementsOnPoint`) 1)
    (set `self.isSprout` true))
  (if (== (`self.movementsOnPoint`) 2)
    (set `self.isWall` true)
    (set `self.isSprout` false))
  (`SceneComponent.SetVisibility` (`self.Wall`) (`self.isWall`) true)
  (`SceneComponent.SetVisibility` (`self.Sprout`) (`self.isSprout`) true)
  ;[1 1 1] If Ice Block
  (if (`self.isIceWall`)
    ;[1 1 1] Lerping Ice Block Scale
    (`SceneComponent.SetRelativeScale3D` _icewall (`KismetMathLibrary.VLerp` (`SceneComponent.RelativeScale3D` _icewall) (`self.TargetScale`) 0.15))
    ;[1 1 1] Lerping UI Position
    (`SceneComponent.K2_SetRelativeLocation` _meltui (`KismetMathLibrary.VLerp` (`SceneComponent.RelativeLocation` _meltui) (`self.UITargetPos`) 0.15) false false)
    ;[1 1 1] Lock Bobbing
    (`self.PlayBobTimeline`)
    ;[1 1 1] Melting Block Checks
    (bind _asbp_player_pawn (cast `/Game/Blueprints/BP_PlayerPawn` (`GameplayStatics.GetPlayerPawn` 0)))
    (if (>= (`/Game/Blueprints/BP_PlayerPawn.movements` _asbp_player_pawn) (`self.maxMovements`))
      (`SceneComponent.SetVisibility` (`self.MeltUI`) false false)
      (`SceneComponent.SetVisibility` (`self.IceWall`) false true)
      (`self.PlayMeltSound`)
      (bind _output_get (set `self.melted` true))
      (if (== (`SceneComponent.RelativeScale3D` (`self.IceWall`)) (`self.TargetScale`) :`ErrorTolerance` 0.005)
        (set `self.isIceWall` false)
        (`SceneComponent.SetVisibility` (`self.IceWall`) (not _output_get) false)
        (`SceneComponent.SetVisibility` (`self.MeltUI`) false false)))))

(event `PlayMeltSound`
  ;[1 1 1] Melt Sound
  (`/Engine/EditorBlueprintResources/StandardMacros.DoOnce` false
    (:`Completed`
      (`GameplayStatics.PlaySound2D` "/Game/Audio/melt.melt" 0.2 1.0 0.0 null null))))

(event `PlayBobTimeline`
  ;[1 1 1] Lock Bobbing Event
  (bind (_direction _moveaxis) (`Timeline|BobTimeline`)
    (:`Update`
      (if (`self.isIceWall`)
        (if (`self.melted`)
          (`SceneComponent.K2_AddWorldOffset` (`self.Lock`) (`KismetMathLibrary.MakeVector` 0.0 0.0 (* _moveaxis (`self.lockBobAmt`))) false false :!label _label))
        (else
          (goto _label))))))

(event `self.ReceiveBeginPlay`
  ;[1 1 1] Setup
  (`self.AssignWidget`)
  (`self.SetIceBlockScale`)
  (if (`self.isIceWall`)
    _))

(fn `AssignWidget`
  (bind _asui_tile_melt (cast `/Game/UserInterface/UI_TileMelt` (`WidgetComponent.GetUserWidgetObject` (`self.MeltUI`))))
  (set `/Game/UserInterface/UI_TileMelt.GridPoint` self _asui_tile_melt))

(fn `Rotate`
  (params (NewParam :type "SceneComponent Object Reference"))
  (bind (_returnvalue_roll _returnvalue_pitch _returnvalue_yaw) (`KismetMathLibrary.BreakRotator` (`SceneComponent.K2_GetComponentRotation` NewParam)))
  (if (not (`self.isIceWall`))
    (`SceneComponent.K2_SetWorldRotation` NewParam (`KismetMathLibrary.MakeRotator` _returnvalue_roll _returnvalue_pitch (+ _returnvalue_yaw (`self.keyRotAmt`))) false false)))

(fn `SetIceBlockScale`
  (bind _meltui (`self.MeltUI`))
  (bind (_relativescale3d_x _relativescale3d_y) (`KismetMathLibrary.BreakVector` (`SceneComponent.RelativeScale3D` (`self.IceWall`))))
  (bind _output_get (set `self.TargetScale` (`KismetMathLibrary.MakeVector` _relativescale3d_x _relativescale3d_y (+ (`self.MinIceScale`) (* (`self.maxMovements`) (`self.IceShrinkScale`))))))
  (`SceneComponent.SetRelativeScale3D` (`self.IceWall`) _output_get)
  (`SceneComponent.K2_SetRelativeLocation` _meltui (`KismetMathLibrary.MakeVector` 0.0 0.0 (+ (* (`self.maxMovements`) (`self.UIMoveAmt`)) 50.0)) false false)
  (set `self.UITargetPos` (`SceneComponent.RelativeLocation` _meltui)))

(fn `SetupGridPoint`
  (bind _issprout (`self.isSprout`))
  (bind _iswall (`self.isWall`))
  (bind _isfinaltile (`self.isFinalTile`))
  (`SceneComponent.SetVisibility` (`self.Lock`) (`self.isLocked`) false)
  (`SceneComponent.SetVisibility` (`self.Key`) (`self.isKeyTile`) false)
  (`SceneComponent.SetVisibility` (`self.Wall`) _iswall true)
  (if _iswall
    (set `self.movementsOnPoint` 2))
  (`SceneComponent.SetVisibility` (`self.Sprout`) _issprout true)
  (if _issprout
    (set `self.movementsOnPoint` 1))
  (`SceneComponent.SetVisibility` (`self.FinalTile`) _isfinaltile true)
  (`SceneComponent.SetVisibility` (`self.Tile`) (not _isfinaltile) false)
  (`SceneComponent.SetVisibility` (`self.IceWall`) (`self.isIceWall`) false)
  (`SceneComponent.SetVisibility` (`self.MeltUI`) (`self.isIceWall`) false)
  (if (not (`self.isFinalTile`))
    (`SceneComponent.SetVisibility` (`self.FinalTile`) (`self.isFinishTile`) false)
    (`SceneComponent.SetVisibility` (`self.Tile`) (not (`self.isFinishTile`)) false)
    (`SceneComponent.SetVisibility` (`self.FinishObject`) (`self.isFinishTile`) true)))

(fn `ShrinkIceBlock`
  (bind (_relativescale3d_x _relativescale3d_y _relativescale3d_z) (`KismetMathLibrary.BreakVector` (`SceneComponent.RelativeScale3D` (`self.IceWall`))))
  (bind (_relativelocation_x _relativelocation_y _relativelocation_z) (`KismetMathLibrary.BreakVector` (`SceneComponent.RelativeLocation` (`self.MeltUI`))))
  (bind (_relativescale3d_x_2 _relativescale3d_y_2) (`KismetMathLibrary.BreakVector` (`SceneComponent.RelativeScale3D` (`self.IceWall`))))
  (set `self.TargetScale` (`KismetMathLibrary.MakeVector` _relativescale3d_x_2 _relativescale3d_y_2 (- _relativescale3d_z (`self.IceShrinkScale`))))
  (set `self.UITargetPos` (`KismetMathLibrary.MakeVector` 0.0 0.0 (- _relativelocation_z (`self.UIMoveAmt`)))))

(fn `UserConstructionScript`
  (`self.SetupGridPoint`)
  (`PrimitiveComponent.SetCastShadow` (`self.MeltUI`) false))